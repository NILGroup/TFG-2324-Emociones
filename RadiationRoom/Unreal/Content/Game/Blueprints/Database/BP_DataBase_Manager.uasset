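; BP_DataBase_Manager is an actor that manages database access for gameplay logging and experiment data.
; On BeginPlay, the authority spawns BP_Database_Server and listens for its closed event, which sets ServerClosed and is rebroadcast.
; CloseDatabase passes through to the server.
; Send and GetUserId events are empty: their forwarding logic to server and local-file databases is disconnected, as is the local-file spawn.
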(event `self.ReceiveBeginPlay`
  (`/Engine/EditorBlueprintResources/ActorMacros.Switch Has Authority`
    (:`Authority`
      (bind _returnvalue (`|SpawnActorFromClass` "/Game/Game/Blueprints/Database/BP_Database_Server.BP_Database_Server_C" (`KismetMathLibrary.MakeTransform` (0.0 0.0 0.0)) "Undefined" "OverrideRootScale" null null))
      (bind _output_get (set `self.ServerDB` _returnvalue))
      (add `/Game/Game/Blueprints/Database/BP_Database_Server.ED_ServerDatabaseClosed` _output_get (delegate `ServerDatabaseClosed`)))))

(event `ServerDatabaseClosed`
  (set `self.ServerClosed` true)
  (`self.ED_DatabaseClosed`))

(event `CloseDatabase`
  (bind _serverdb (`self.ServerDB`)
    (:`then`
      (`/Game/Game/Blueprints/Database/BP_Database_Server.CloseDatabase` _serverdb))
    (:`else`)))

(event `Send Interact Event to DB`
  (params (Data :type "/Game/Game/DataStructures/Database/F_InteractEventsTableItem Structure")))

(event `Send Gameplay Event to DB`
  (params (Data :type "/Game/Game/DataStructures/Database/F_GameplayEventsTableItem Structure")))

(event `Send User to DB`
  (params (Data :type "/Game/Game/DataStructures/Database/F_UserTableItem Structure")))

(event `Send Team to DB`
  (params (Data :type "/Game/Game/DataStructures/Database/F_TeamTableItem Structure")))

(event `Send Session to DB`
  (params (Data :type "/Game/Game/DataStructures/Database/F_SessionTableItem Structure")))

(event `Send Experiment to DB`
  (params (Data :type "/Game/Game/DataStructures/Database/F_ExperimentTableItem Structure")))

(event `Get User Id`
  (params (`Player Name` :type String)))

(event `Send Move Event to DB`
  (params (Data :type "/Game/Game/DataStructures/Database/F_MoveEventsTableItem Structure")))

(fn `UserConstructionScript`)