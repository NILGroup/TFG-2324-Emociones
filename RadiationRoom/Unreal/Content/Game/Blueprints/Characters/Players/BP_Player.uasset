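; Networked player for a training game that handles item and NPC interaction, widget HUDs and logging of player activity to a database.
; Look-at detection line-traces from several components, picks the most-hit interactable, then sends interface messages for look-at, interact, use and cancel through OnServer-to-Multi event pairs.
; BeginPlay links the database manager, gameplay manager and phase, countdown and end-screen widgets.
; Movement start and stop are timed, with sampled distance saved as move events.
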(event `self.ReceiveBeginPlay`
  (bind _returnvalue (`GameplayStatics.GetActorOfClass` "/Game/Game/Blueprints/Database/BP_DataBase_Manager.BP_DataBase_Manager_C"))
  (`self.Set DB On Server` _returnvalue)
  (if (`self.IsLocallyControlled`)
    (`|ExecutionSequence`
      (:`then_0`
        (`self.Set HUD On Server`))
      (:`then_1`
        (bind _asrr_game_instance (cast `/Game/Game/Blueprints/RR_GameInstance` (`GameplayStatics.GetGameInstance`)))
        (set `self.UserId` (`/Game/Game/Blueprints/RR_GameInstance.PlayerID` _asrr_game_instance))
        (set `self.Name` (`/Game/Game/Blueprints/RR_GameInstance.PlayerName` _asrr_game_instance)))
      (:`then_2`
        (bind _dbmanager (`self.DBManager`)
          (:`then`
            (`/Game/Game/Blueprints/Database/BP_DataBase_Manager.Send Gameplay Event to DB` _dbmanager (make `/Game/Game/DataStructures/Database/F_GameplayEventsTableItem` 0 (`self.UserId`) "NewEnumerator0" "NewEnumerator9" (`KismetMathLibrary.Now`))))
          (:`else`)))
      (:`then_3`
        (`self.StartToPlay`))
      (:`then_4`
        (bind _output_get (set `self.CurrentPosition` (`self.K2_GetActorLocation`)))
        (set `self.InitialPosition` _output_get)))))

(event `self.ReceiveTick`
  (params (DeltaSeconds :type "Float (single-precision)")))

(event `StartToPlay`
  (bind _returnvalue (`GameplayStatics.GetCurrentLevelName` true))
  (if (and (`KismetStringLibrary.NotEqual_StrStr` _returnvalue "MainMenuMap") (`KismetStringLibrary.NotEqual_StrStr` _returnvalue "DevelopMap"))
    (`GameplayStatics.PlaySound2D` "/Game/Game/Blueprints/Audio/SC_AmbientSound.SC_AmbientSound" 0.5 1.0 0.0 null null)
    (bind _asplayer_controller (cast `PlayerController` (`self.GetController`)))
    (`self.EnableInput` _asplayer_controller)
    (`KismetSystemLibrary.Delay` 2.0)
    (bind _gameplaymanager (`self.GameplayManager`)
      (:`then`
        (`|ExecutionSequence`
          (:`then_0`
            (bind _phaseshud (`self.PhasesHUD`)
              (:`then`
                (`/Game/Game/Blueprints/Gameplay/BP_GameplayManager.SetPhasesHUD` _gameplaymanager _phaseshud))
              (:`else`)))
          (:`then_1`
            (bind _theendhud (`self.TheEndHUD`)
              (:`then`
                (`/Game/Game/Blueprints/Gameplay/BP_GameplayManager.SetTheEndHUD` _gameplaymanager _theendhud))
              (:`else`)))))
      (:`else`))))

(event `Key|L`
  (params (Key :type "Key Structure"))
  (:`Pressed`
    (bind _dbmanager (`self.DBManager`)
      (:`then`
        (`/Game/Game/Blueprints/Database/BP_DataBase_Manager.Send Gameplay Event to DB` _dbmanager (make `/Game/Game/DataStructures/Database/F_GameplayEventsTableItem` 0 (`self.UserId`) "NewEnumerator0" "NewEnumerator7" (`KismetMathLibrary.Now`)))
        (`KismetSystemLibrary.Delay` 0.5)
        (bind _asrr_game_instance (cast `/Game/Game/Blueprints/RR_GameInstance` (`GameplayStatics.GetGameInstance`)))
        (`/Game/Game/Blueprints/RR_GameInstance.CloseDatabase` _asrr_game_instance))
      (:`else`))))

(event `AddDistance`
  (bind _returnvalue (+ (`KismetMathLibrary.Vector_Distance` (`self.LocationMove`) (`SceneComponent.K2_GetComponentLocation` (`self.Mesh`))) (`self.Distance Move`)))
  (if (`self.IsMoving`)
    (if (> _returnvalue 50.0)
      (set `self.Distance Move` _returnvalue)
      (set `self.LocationMove` (`SceneComponent.K2_GetComponentLocation` (`self.Mesh`))))
    (`KismetSystemLibrary.Delay` 0.2)
    (`self.AddDistance`)))

(event `PlayerIsMoving`
  (params (`Axis value` :type "Float (double-precision)"))
  (if (!= `Axis value` 0.0)
    (if (not (`self.IsMoving`))
      (set `self.IsMoving` true)
      (set `self.Start Datetime Move` (`KismetMathLibrary.Now`))
      (bind _output_get (set `self.Start Position Move` (`SceneComponent.K2_GetComponentLocation` (`self.Mesh`))))
      (set `self.LocationMove` _output_get)
      (set `self.Distance Move` 0.0)
      (`self.AddDistance`))
    (elif (`self.IsMoving`)
      (set `self.IsMoving` false)
      (set `self.End Datetime Move` (`KismetMathLibrary.Now`))
      (bind _output_get_2 (set `self.End Position Move` (`SceneComponent.K2_GetComponentLocation` (`self.Mesh`))))
      (set `self.CurrentPosition` _output_get_2)
      (set `self.Distance Move` (+ (`KismetMathLibrary.Vector_Distance` (`self.LocationMove`) (`self.End Position Move`)) (`self.Distance Move`)))
      (bind _dbmanager (`self.DBManager`)
        (:`then`
          (`/Game/Game/Blueprints/Database/BP_DataBase_Manager.Send Move Event to DB` _dbmanager (make `/Game/Game/DataStructures/Database/F_MoveEventsTableItem` 0 (`self.UserId`) "NewEnumerator0" "NewEnumerator1" (`self.Start Datetime Move`) (`self.End Datetime Move`) (`self.Start Position Move`) (`self.End Position Move`) (/ (`self.Distance Move`) 100.0))))
        (:`else`)))))

(event `Check Look At On Server`
  (params (Player :type "/Game/Game/Blueprints/Characters/Players/BP_Player Object Reference") (`Look from Component` :type "Array of SceneComponent Object Reference"))
  ;[1 1 1] Check Look At
  (`self.Check Look At Multi` Player `Look from Component`))

(event `Check Look At Multi`
  (params (Player :type "/Game/Game/Blueprints/Characters/Players/BP_Player Object Reference") (`Look from Component` :type "Array of SceneComponent Object Reference"))
  ;[1 1 1] Check Look At
  (bind _look_at_actor (`self.CheckLookAt` Player `Look from Component`))
  (if (!= _look_at_actor (`/Game/Game/Blueprints/Characters/Players/BP_Player.LookAtActor` Player))
    (`self.Look At Nothing` Player)
    (`/Engine/EditorBlueprintResources/StandardMacros.IsValid` _look_at_actor
      (:`Is Valid`
        (bind _output_get (set `/Game/Game/Blueprints/Characters/Players/BP_Player.LookAtActor` _look_at_actor Player))
        (bind _asbp_interact_item_parent (cast `/Game/Game/Blueprints/Actors/Items/BP_InteractItemParent` _output_get)
          (:`then`
            (`self.Look At Interact Item` _asbp_interact_item_parent Player))
          (:`CastFailed`
            (bind _asbp_npc_talkable (cast `/Game/Game/Blueprints/Characters/AI/BP_NPC_Talkable` _output_get)
              (:`then`
                (`self.Look At Interact NPC` _asbp_npc_talkable Player))
              (:`CastFailed`
                (bind _asbp_place_point (cast `/Game/Game/Blueprints/Actors/Items/UsePoints/PlacePoints/BP_PlacePoint` _output_get))
                (`self.Look At Place Point` _asbp_place_point Player)))))))))

(event `Look At Nothing`
  (params (Player :type "/Game/Game/Blueprints/Characters/Players/BP_Player Object Reference"))
  ;[1 1 1] Check Look At
  (bind _lookatactor (`/Game/Game/Blueprints/Characters/Players/BP_Player.LookAtActor` Player)
    (:`then`
      (message `/Game/Game/Blueprints/Interfaces/BI_Interact.StopLookAt` _lookatactor Player)
      (set `/Game/Game/Blueprints/Characters/Players/BP_Player.LookAtActor` null Player))
    (:`else`)))

(event `Look At Interact Item`
  (params (Item :type "/Game/Game/Blueprints/Actors/Items/BP_InteractItemParent Object Reference") (Player :type "/Game/Game/Blueprints/Characters/Players/BP_Player Object Reference"))
  ;[1 1 1] Check Look At
  (message `/Game/Game/Blueprints/Interfaces/BI_Interact.StartLookAt` Item Player))

(event `Look At Interact NPC`
  (params (NPC :type "/Game/Game/Blueprints/Characters/AI/BP_NPC_Talkable Object Reference") (Player :type "/Game/Game/Blueprints/Characters/Players/BP_Player Object Reference"))
  ;[1 1 1] Check Look At
  (message `/Game/Game/Blueprints/Interfaces/BI_Interact.StartLookAt` NPC Player))

(event `Look At Place Point`
  (params (`Place Point` :type "/Game/Game/Blueprints/Actors/Items/UsePoints/PlacePoints/BP_PlacePoint Object Reference") (Player :type "/Game/Game/Blueprints/Characters/Players/BP_Player Object Reference"))
  ;[1 1 1] Check Look At
)

(event `Interact With On Server`
  (params (`Look At Actor` :type "Actor Object Reference") (Player :type "/Game/Game/Blueprints/Characters/Players/BP_Player Object Reference"))
  ;[1 1 1] Interact with
  (`/Engine/EditorBlueprintResources/StandardMacros.IsValid` `Look At Actor`
    (:`Is Valid`
      (`self.Interact With Multi` `Look At Actor` Player))))

(event `Use On Server`
  (params (Actor :type "Actor Object Reference") (Point :type "Actor Object Reference") (Player :type "/Game/Game/Blueprints/Characters/Players/BP_Player Object Reference"))
  ;[1 1 1] Interact with
  (`/Engine/EditorBlueprintResources/StandardMacros.IsValid` Actor
    (:`Is Valid`
      (`self.Use Multi` Actor Point Player))))

(event `Interact With Multi`
  (params (`Look At Actor` :type "Actor Object Reference") (Player :type "/Game/Game/Blueprints/Characters/Players/BP_Player Object Reference"))
  ;[1 1 1] Interact with
  (`/Engine/EditorBlueprintResources/StandardMacros.IsValid` `Look At Actor`
    (:`Is Valid`
      (message `/Game/Game/Blueprints/Interfaces/BI_Interact.InteractWith` `Look At Actor` Player))))

(event `Use Multi`
  (params (Actor :type "Actor Object Reference") (Point :type "Actor Object Reference") (Player :type "/Game/Game/Blueprints/Characters/Players/BP_Player Object Reference"))
  ;[1 1 1] Interact with
  (`/Engine/EditorBlueprintResources/StandardMacros.IsValid` Actor
    (:`Is Valid`
      (message `/Game/Game/Blueprints/Interfaces/BI_Interact.UseWith` Actor Point Player))))

(event `Cancel On Server`
  (params (Item :type "/Game/Game/Blueprints/Actors/Items/BP_InteractItemParent Object Reference") (Player :type "/Game/Game/Blueprints/Characters/Players/BP_Player Object Reference"))
  ;[1 1 1] Cancel Interact
  (`self.Cancel Multi` Item Player))

(event `Cancel Multi`
  (params (Item :type "/Game/Game/Blueprints/Actors/Items/BP_InteractItemParent Object Reference") (Player :type "/Game/Game/Blueprints/Characters/Players/BP_Player Object Reference"))
  ;[1 1 1] Cancel Interact
  (message `/Game/Game/Blueprints/Interfaces/BI_Interact.CancelInteract` Item Player)
  (set `self.CurrentHeldItem` null))

(event `WearDosimeter`)

(event `Set HUD On Server`
  ;[1 1 1] Set HUD
  (`self.Set HUD On Client`))

(event `Set HUD On Client`
  (bind _countdowntimerwidget (`self.CountdowntimerWidget`))
  (bind _theendwidget (`self.TheEndWidget`))
  ;[1 1 1] Set HUD
  (bind _asplayer_controller (cast `PlayerController` (`self.GetController`)))
  (`|ExecutionSequence`
    (:`then_0`
      (bind _asrr_hud (cast `/Game/Game/Blueprints/UI/RR_HUD` (`PlayerController.GetHUD` _asplayer_controller)))
      (set `self.HUD` _asrr_hud)
      (bind _returnvalue (`GameplayStatics.GetActorOfClass` "/Game/Game/Blueprints/Gameplay/BP_GameplayManager.BP_GameplayManager_C"))
      (`self.Set GameplayManager On Server ` _returnvalue)
      (bind _gameplaymanager (`self.GameplayManager`)
        (:`then`
          (set `/Game/Game/Blueprints/Gameplay/BP_GameplayManager.Player` self _gameplaymanager))
        (:`else`)))
    (:`then_1`
      (`SceneComponent.SetVisibility` _theendwidget false false)
      (bind _aswbp_the_end (cast `/Game/Game/Blueprints/UI/TheEnd/WBP_TheEnd` (`WidgetComponent.GetWidget` _theendwidget)))
      (set `self.TheEndHUD` _aswbp_the_end)
      (bind _gameplaymanager_2 (`self.GameplayManager`)
        (:`then`
          (add `/Game/Game/Blueprints/Gameplay/BP_GameplayManager.GameplayIsCompleted` _gameplaymanager_2 (delegate `GameplayCompleted`)))
        (:`else`)))
    (:`then_2`
      (`SceneComponent.SetVisibility` _countdowntimerwidget false false)
      (bind _aswbp_countdown_timer (cast `/Game/Game/Blueprints/UI/WBP_CountdownTimer` (`WidgetComponent.GetWidget` _countdowntimerwidget)))
      (set `self.CountdownTimerHUD` _aswbp_countdown_timer))
    (:`then_3`
      (bind _gameplaymanager_3 (`self.GameplayManager`)
        (:`then`
          (if (not (`/Game/Game/Blueprints/Gameplay/BP_GameplayManager.FreeTraining` _gameplaymanager_3))
            (bind _aswbp_phases (cast `/Game/Game/Blueprints/UI/WBP_Phases` (`WidgetComponent.GetWidget` (`self.PhasesWidget`))))
            (set `self.PhasesHUD` _aswbp_phases)))
        (:`else`)))))

(event `GameplayCompleted`
  ;[1 1 1] Set HUD
  (`SceneComponent.SetVisibility` (`self.TheEndWidget`) true false)
  (`/Game/Game/Blueprints/UI/TheEnd/WBP_TheEnd.CheckCompletedPhases` (`self.TheEndHUD`) (`/Game/Game/Blueprints/Gameplay/BP_GameplayManager.Objectives` (`self.GameplayManager`)))
  (set `self.IsGameplayCompleted` true))

(event `Set Name On Server`
  (params (Name :type String))
  (if (`KismetStringLibrary.NotEqual_StrStr` Name)
    (set `self.Name` Name)))

(event `SetIdOnServer`
  (params (Id :type Integer))
  (set `self.UserId` Id))

(event `Get User Id`
  (bind _dbmanager (`self.DBManager`)
    (:`then`
      (`/Game/Game/Blueprints/Database/BP_DataBase_Manager.Get User Id` _dbmanager (`self.Name`)))
    (:`else`)))

(event `Set Player Color On Server`
  (params (Color :type "LinearColor Structure"))
  (set `self.Color` Color))

(event `Set DB On Server`
  (params (DataBase :type "/Game/Game/Blueprints/Database/BP_DataBase_Manager Object Reference"))
  (`self.Set DB On Client` DataBase))

(event `Set DB On Client`
  (params (DataBase :type "/Game/Game/Blueprints/Database/BP_DataBase_Manager Object Reference"))
  (set `self.DBManager` DataBase))

(event `Set GameplayManager On Server`
  (params (GameplayManager :type "/Game/Game/Blueprints/Gameplay/BP_GameplayManager Object Reference"))
  (`self.Set GameplayManager On Client` GameplayManager))

(event `Set GameplayManager On Client`
  (params (GameplayManager :type "/Game/Game/Blueprints/Gameplay/BP_GameplayManager Object Reference"))
  (set `self.GameplayManager` GameplayManager))

(fn `CheckLookAt`
  (params (Player :type "/Game/Game/Blueprints/Characters/Players/BP_Player Object Reference") (`Look from Component` :type "Array of SceneComponent Object Reference") (`Show Laser` :type Boolean :default false))
  (returns (`Look at Actor` :type "Actor Object Reference"))
  (locals (ShowLaser :type "EDrawDebugTrace Enum" :default "ForOneFrame") (HitActors :type "Array of Actor Object Reference") (HitActorsTimes :type "Array of Integer"))
  (bind _hitactorstimes (`local.HitActorsTimes`))
  (for _array_element `Look from Component`
    (bind (_startpoint _endpoint) (`self.LookHitPoint` Player _array_element 250.0))
    (if `Show Laser`
      (set `local.ShowLaser` "ForOneFrame")
      (else
        (set `local.ShowLaser` "None")))
    (bind _outhit (`KismetSystemLibrary.LineTraceSingle` :`Start` _startpoint :`End` _endpoint :`TraceChannel` "TraceTypeQuery2" :`DrawDebugType` (`local.ShowLaser`)))
    (if (or (`KismetSystemLibrary.DoesImplementInterface` (`.HitActor` (`GameplayStatics.BreakHitResult` _outhit)) "/Game/Game/Blueprints/Interfaces/BI_Interact.BI_Interact_C") (`KismetSystemLibrary.DoesImplementInterface` (`.HitActor` (`GameplayStatics.BreakHitResult` _outhit)) "/Game/Game/Blueprints/Interfaces/BI_Use.BI_Use_C"))
      (bind _returnvalue (`KismetArrayLibrary.Array_Find` (`local.HitActors`) (`.HitActor` (`GameplayStatics.BreakHitResult` _outhit))))
      (if (!= _returnvalue -1)
        (`KismetArrayLibrary.Array_Set` _hitactorstimes _returnvalue (+ (`|GetArrayItem` _hitactorstimes _returnvalue) 1))
        (else
          (`KismetArrayLibrary.Array_Add` (`local.HitActors`) (`.HitActor` (`GameplayStatics.BreakHitResult` _outhit)))
          (`KismetArrayLibrary.Array_Add` (`local.HitActorsTimes`))))))
  (if (> (`KismetArrayLibrary.Array_Length` (`local.HitActors`)) 0)
    (return (`|GetArrayItem` (`local.HitActors`) (`KismetMathLibrary.MaxOfIntArray` (`local.HitActorsTimes`))))
    (else
      (return null))))

(fn `LookHitPoint`
  (params (`From Component` :type "SceneComponent Object Reference") (Distance :type "Float (double-precision)"))
  (returns (StartPoint :type "Vector Structure") (EndPoint :type "Vector Structure"))
  (bind _returnvalue (`SceneComponent.K2_GetComponentLocation` `From Component`))
  (return _returnvalue (+ _returnvalue (* (`KismetMathLibrary.GetForwardVector` (`SceneComponent.K2_GetComponentRotation` `From Component`)) Distance))))

(fn `OnRep_Color`
  (bind _returnvalue (`PrimitiveComponent.CreateDynamicMaterialInstance` (`self.Mesh`) 0 "/Game/Game/Materials/M_MaleCharacter.M_MaleCharacter" "None"))
  (`MaterialInstanceDynamic.SetVectorParameterValue` _returnvalue "BodyColor" (`self.Color`)))

(fn `OnRep_Name`
  (`TextRenderComponent.K2_SetText` (`self.PlayerName`) (`KismetTextLibrary.Conv_StringToText` (`self.Name`))))

(fn `UserConstructionScript`)